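; Base laser turret that can follow a spline path and detects actors carrying a TurretDetectableComponent.
; Each tick it moves, rotates by its RotationType or snaps to the locked target, then traces and stretches the laser mesh to the hit.
; A lock starts a timeline color charge that fires damage traces and repeats while locked.
; Detection, loss and damage go through the GameMaster; Make*LaserArray functions wrap traces as arrays.
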(event `self.ReceiveBeginPlay`
  (`self.SetupPath`)
  (`self.SetupLaserEnds` (`|MakeArray` (`self.laserEnd`)))
  (set `self.InitialRotation` (`SceneComponent.K2_GetComponentRotation` (`self.DefaultSceneRoot`))))

(event `self.ReceiveTick`
  (params (DeltaSeconds :type "Float (single-precision)"))
  (`self.MoveAlongSpline`)
  (`self.RotateTurret`)
  (bind _results (`self.MakeDetectionLaserArray`))
  (`self.AimForDetectable` _results))

(event `ChargeLaserShot`
  (bind (_direction _alpha) (`Timeline|LaserColorLerpAlpha` :!via `PlayFromStart` :!label _label)
    (:`Update`
      (`MeshComponent.SetScalarParameterValueOnMaterials` (`self.Plane`) "ColorLerp" _alpha)
      (if (not (`self.LockedOnTarget`))
        (`MeshComponent.SetScalarParameterValueOnMaterials` (`self.Plane`) "ColorLerp" 0.01)
        (goto _label :!via `Stop`)))
    (:`Finished`
      (bind _hits (`self.MakeDamageLaserArray`))
      (`self.DamageLasersHits` _hits)
      (if (`self.LockedOnTarget`)
        (`self.ChargeLaserShot`)
        (else
          (`MeshComponent.SetScalarParameterValueOnMaterials` (`self.Plane`) "ColorLerp" 0.01))))))

(fn `AimForDetectable`
  (params (OutHits :type "Array of HitResult Structure"))
  (locals (hasTargetOnSight :type Boolean :default false))
  (for _array_element OutHits
    (bind (_bblockinghit _binitialoverlap _time _distance _location _impactpoint _normal _impactnormal _physmat _hitactor) (`GameplayStatics.BreakHitResult` _array_element))
    (if (`KismetSystemLibrary.IsValid` _hitactor)
      (if (not (`self.LockedOnTarget`))
        (bind _returnvalue (`self.GetComponentByClass` _hitactor "/Game/Blueprints/Components/TurretDetectableComponent.TurretDetectableComponent_C"))
        (if (`KismetSystemLibrary.IsValid` _returnvalue)
          (bind _output_get (set `self.LockedDetectable` _returnvalue))
          (set `self.LockedOnTarget` true)
          (set `local.hasTargetOnSight` true)
          (`self.ChargeLaserShot`)
          (`/Game/Blueprints/GameMaster/GameMaster.OnTurretDectectedObject` (`/Game/Blueprints/Libraries/CommonLibrary.GetGameMaster`) _output_get self))
        (else
          (bind _returnvalue_2 (`self.GetComponentByClass` _hitactor "/Game/Blueprints/Components/TurretDetectableComponent.TurretDetectableComponent_C"))
          (if (`KismetSystemLibrary.IsValid` _returnvalue_2)
            (if (== _returnvalue_2 (`self.LockedDetectable`))
              (set `local.hasTargetOnSight` true)))))))
  (if (not (`self.LockedOnTarget`))
    _
    (elif (not (`local.hasTargetOnSight`))
      (`/Game/Blueprints/GameMaster/GameMaster.OnTurretLostObject` (`/Game/Blueprints/Libraries/CommonLibrary.GetGameMaster`) (`self.LockedDetectable`) self)
      (set `self.LockedDetectable` null)
      (set `self.LockedOnTarget` false))))

(fn `CastDamageLaser`
  (params (Start :type "SceneComponent Object Reference"))
  (returns (HitResult :type "HitResult Structure"))
  (bind _returnvalue (`SceneComponent.K2_GetComponentLocation` Start))
  (bind _outhit (`KismetSystemLibrary.LineTraceSingleForObjects` :`Start` _returnvalue :`End` (+ _returnvalue (* (`SceneComponent.GetForwardVector` Start) (`self.LaserLength`))) :`ObjectTypes` (`|MakeArray` "ObjectTypeQuery3" "ObjectTypeQuery1" "ObjectTypeQuery2" "ObjectTypeQuery4" "ObjectTypeQuery7" :!type "EObjectTypeQuery Enum") :`TraceColor` (struct :`G` 1.0 :`B` 0.330944 :`A` 1.0) :`TraceHitColor` (struct :`G` 0.815726 :`B` 1.0 :`A` 1.0)))
  (return _outhit))

(fn `CastDetectionLaser`
  (params (Start :type "SceneComponent Object Reference") (End :type "SceneComponent Object Reference") (LaserMesh :type "SceneComponent Object Reference"))
  (returns (HitResult :type "HitResult Structure"))
  (locals (EndPosition :type "Vector Structure"))
  (bind _returnvalue (`SceneComponent.K2_GetComponentLocation` Start))
  (bind _returnvalue_2 (`SceneComponent.K2_GetComponentLocation` End))
  (bind _returnvalue_3 (`SceneComponent.K2_GetComponentLocation` Start))
  (bind (_relativescale3d_x _relativescale3d_y) (`KismetMathLibrary.BreakVector` (`SceneComponent.RelativeScale3D` LaserMesh)))
  (bind (_outhit _returnvalue_4) (`KismetSystemLibrary.LineTraceSingleForObjects` :`Start` _returnvalue :`End` (+ _returnvalue (* (`SceneComponent.GetForwardVector` Start) (`self.LaserLength`))) :`ObjectTypes` (`|MakeArray` "ObjectTypeQuery3" "ObjectTypeQuery1" "ObjectTypeQuery2" "ObjectTypeQuery4" "ObjectTypeQuery7" :!type "EObjectTypeQuery Enum") :`TraceColor` (struct :`G` 1.0 :`B` 0.330944 :`A` 1.0) :`TraceHitColor` (struct :`G` 0.815726 :`B` 1.0 :`A` 1.0)))
  (if _returnvalue_4
    (bind (_bblockinghit _binitialoverlap _time _distance _location _impactpoint _normal _impactnormal _physmat _hitactor _hitcomponent _hitbonename _hititem _faceindex _tracestart _traceend) (`GameplayStatics.BreakHitResult` _outhit))
    (set `local.EndPosition` _impactpoint)
    (else
      (set `local.EndPosition` _traceend)))
  (`SceneComponent.K2_SetWorldLocation` End (`local.EndPosition`) false false)
  (`SceneComponent.K2_SetWorldLocation` LaserMesh (`KismetMathLibrary.VLerp` _returnvalue_3 _returnvalue_2 0.5) false false)
  (`SceneComponent.SetRelativeScale3D` LaserMesh (`KismetMathLibrary.MakeVector` _relativescale3d_x _relativescale3d_y (+ (* (`KismetMathLibrary.Vector_Distance` _returnvalue_3 _returnvalue_2) 0.01) 0.05)))
  (return _outhit))

(fn `DamageLasersHits`
  (params (Hits :type "Array of HitResult Structure"))
  (for _array_element Hits
    (bind (_bblockinghit _binitialoverlap _time _distance _location _impactpoint _normal _impactnormal _physmat _hitactor) (`GameplayStatics.BreakHitResult` _array_element))
    (`/Engine/EditorBlueprintResources/StandardMacros.IsValid` _hitactor
      (:`Is Valid`
        (`/Game/Blueprints/GameMaster/GameMaster.OnDamageDealt` (`/Game/Blueprints/Libraries/CommonLibrary.GetGameMaster`) self _hitactor (`self.LaserDamages`))))))

(fn `MakeDamageLaserArray`
  (returns (Hits :type "Array of HitResult Structure"))
  (bind _hitresult (`self.CastDamageLaser` (`self.LaserMuzzle`)))
  (return (`|MakeArray` _hitresult)))

(fn `MakeDetectionLaserArray`
  (returns (Results :type "Array of HitResult Structure"))
  (bind _hitresult (`self.CastDetectionLaser` (`self.LaserMuzzle`) (`self.laserEnd`) (`self.Plane`)))
  (return (`|MakeArray` _hitresult)))

(fn `MoveAlongSpline`
  (if (`self.FollowSpline`)
    (bind _output_get (set `self.CurrentSplineTime` (+ (`self.CurrentSplineTime`) (* (`self.MovementSpeed`) (`GameplayStatics.GetWorldDeltaSeconds`)))))
    (if (> _output_get 1.0)
      (set `self.CurrentSplineTime` 0.0))
    (`SceneComponent.K2_SetWorldLocation` (`self.DefaultSceneRoot`) (`SplineComponent.GetLocationAtTime` (`self.Path`) (`self.CurrentSplineTime`) "World" false) false false)))

(fn `ResetSpline`
  (`SceneComponent.K2_SetRelativeLocation` (`self.Path`) (0.0 0.0 0.0) false false)
  (`SplineComponent.ClearSplinePoints` (`self.Path`) true)
  (`SplineComponent.AddPoint` (`self.Path`) (make `SplinePoint` 0.0) true)
  (`SplineComponent.AddPoint` (`self.Path`) (make `SplinePoint` 1.0 (100.0 0.0 0.0)) true))

(fn `RotateTurret`
  (locals (Rotation :type "Rotator Structure"))
  (bind _defaultsceneroot (`self.DefaultSceneRoot`))
  (bind (_returnvalue_x _returnvalue_y _returnvalue_z) (`KismetMathLibrary.BreakVector` (* (`self.RotationAxis`) (`self.RotationLerpingSpeed`))))
  (if (`self.LockedOnTarget`)
    ;[1 1 1] Look at target if locked
    (`SceneComponent.K2_SetWorldRotation` _defaultsceneroot (`KismetMathLibrary.FindLookAtRotation` (`SceneComponent.K2_GetComponentLocation` _defaultsceneroot) (`SceneComponent.K2_GetComponentLocation` (`/Game/Blueprints/Components/TurretDetectableComponent.Target` (`self.LockedDetectable`)))) false false)
    (else
      (`|ExecutionSequence`
        (:`then_0`
          (switch `/Game/Blueprints/Turrets/TurretRotationType` (`self.RotationType`)
            (:`NewEnumerator0`
              (set `local.Rotation` (`KismetMathLibrary.RInterpTo` (`SceneComponent.K2_GetComponentRotation` (`self.DefaultSceneRoot`)) (`self.InitialRotation`) (`GameplayStatics.GetWorldDeltaSeconds`) (`self.RotationLerpingSpeed`)))
              (`SceneComponent.K2_SetWorldRotation` (`self.DefaultSceneRoot`) (`local.Rotation`) false false))
            (:`NewEnumerator1`
              (set `local.Rotation` (`KismetMathLibrary.RInterpTo` (`SceneComponent.K2_GetComponentRotation` (`self.DefaultSceneRoot`)) (`KismetMathLibrary.FindLookAtRotation` (`SceneComponent.K2_GetComponentLocation` (`self.DefaultSceneRoot`)) (`self.K2_GetActorLocation` (`self.LookAtTarget`))) (`GameplayStatics.GetWorldDeltaSeconds`) (`self.RotationLerpingSpeed`)))
              (`SceneComponent.K2_SetWorldRotation` (`self.DefaultSceneRoot`) (`local.Rotation`) false false))
            (:`NewEnumerator2`
              (set `local.Rotation` (`KismetMathLibrary.RInterpTo` (`SceneComponent.K2_GetComponentRotation` (`self.DefaultSceneRoot`)) (`KismetMathLibrary.FindLookAtRotation` (`SceneComponent.K2_GetComponentLocation` (`self.DefaultSceneRoot`)) (`SplineComponent.GetLocationAtTime` (`self.Path`) (+ (`self.CurrentSplineTime`) 0.01) "World" false)) (`GameplayStatics.GetWorldDeltaSeconds`) (`self.RotationLerpingSpeed`)))
              (`SceneComponent.K2_SetWorldRotation` (`self.DefaultSceneRoot`) (`local.Rotation`) false false))
            (:`NewEnumerator3`
              (`SceneComponent.K2_AddWorldRotation` (`self.DefaultSceneRoot`) (`KismetMathLibrary.MakeRotator` _returnvalue_x _returnvalue_y _returnvalue_z) false false))))))))

(fn `SetupLaserEnds`
  (params (Ends :type "Array of SceneComponent Object Reference"))
  (for _array_element Ends
    (`SceneComponent.K2_DetachFromComponent` _array_element "KeepWorld" "KeepRelative" "KeepWorld" true)))

(fn `SetupPath`
  (`SceneComponent.K2_DetachFromComponent` (`self.Path`) "KeepWorld" "KeepWorld" "KeepWorld" true))

(fn `UserConstructionScript`
  (`self.CastDetectionLaser` (`self.LaserMuzzle`) (`self.laserEnd`) (`self.Plane`)))