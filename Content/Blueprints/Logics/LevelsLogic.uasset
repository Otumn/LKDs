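; Level-flow logic Blueprint that switches maps when the GameMaster broadcasts next level, replay or main menu events.
; On BeginPlay it binds its handlers to those GameMaster dispatchers.
; Next level increments the GameMaster's CurrentLevelIndex and opens that LevelList entry by name, returning to the menu past the list's end.
; Replay reopens the current level, while main menu resets the index and opens TestMap.
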(event `self.ReceiveBeginPlay`
  (`self.SetupEvents`))

(event `OnNextLevel`
  (bind _result (`/Engine/EditorBlueprintResources/StandardMacros.IncrementInt` (`/Game/Blueprints/GameMaster/GameMaster.CurrentLevelIndex` (`/Game/Blueprints/Libraries/CommonLibrary.GetGameMaster`)))
    (:`  `
      (if (> _result (- (`KismetArrayLibrary.Array_Length` (`self.LevelList`)) 1))
        (`self.OnMainMenu`)
        (else
          (`GameplayStatics.OpenLevel` (`KismetStringLibrary.Conv_StringToName` (`|GetArrayItem` (`self.LevelList`) _result))))))))

(event `OnReplayLevel`
  (bind _returnvalue (`GameplayStatics.GetCurrentLevelName` true))
  (`GameplayStatics.OpenLevel` (`KismetStringLibrary.Conv_StringToName` _returnvalue)))

(event `OnMainMenu`
  (set `/Game/Blueprints/GameMaster/GameMaster.CurrentLevelIndex` 0 (`/Game/Blueprints/Libraries/CommonLibrary.GetGameMaster`))
  (`GameplayStatics.OpenLevel` "TestMap"))

(fn `SetupEvents`
  (add `/Game/Blueprints/GameMaster/GameMaster.OnGoToNextLevel` (`/Game/Blueprints/Libraries/CommonLibrary.GetGameMaster`) (`|CreateDelegate` :!event `OnNextLevel`))
  (add `/Game/Blueprints/GameMaster/GameMaster.OnGoToMainMenu` (`/Game/Blueprints/Libraries/CommonLibrary.GetGameMaster`) (`|CreateDelegate` :!event `OnMainMenu`))
  (add `/Game/Blueprints/GameMaster/GameMaster.OnReplayLevel` (`/Game/Blueprints/Libraries/CommonLibrary.GetGameMaster`) (`|CreateDelegate` :!event `OnReplayLevel`)))

(fn `UserConstructionScript`)