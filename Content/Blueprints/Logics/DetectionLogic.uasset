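; DetectionLogic tracks which detectable objects the turrets currently see, driven by GameMaster events bound on BeginPlay.
; AllDetectedObjects holds one entry per detection, acting as a reference count, while DetectedObjectSingles holds each object once.
; Each loss removes one entry; when none remain, the object leaves the singles list and GameMaster's all-turrets-lost event fires.
; Its own all-turrets-lost handler is empty.
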(event `self.ReceiveBeginPlay`
  (`self.SetupEvents`))

(event `OnObjectDetected`
  (params (Detectable :type "/Game/Blueprints/Components/TurretDetectableComponent Object Reference") (Turret :type "/Game/Blueprints/Turrets/BaseTurret Object Reference"))
  (`self.AddDetectedObject` Detectable))

(event `OnObjectLost`
  (params (Detectable :type "/Game/Blueprints/Components/TurretDetectableComponent Object Reference") (Turret :type "/Game/Blueprints/Turrets/BaseTurret Object Reference"))
  (`self.RemoveDetectedObject` Detectable Turret))

(event `OnAllTurretsLosrtObject`
  (params (Detectable :type "/Game/Blueprints/Components/TurretDetectableComponent Object Reference") (LastTurret :type "/Game/Blueprints/Turrets/BaseTurret Object Reference")))

(fn `AddDetectedObject`
  (params (Object :type "/Game/Blueprints/Components/TurretDetectableComponent Object Reference"))
  (`KismetArrayLibrary.Array_Add` (`self.AllDetectedObjects`) Object)
  (if (not (`KismetArrayLibrary.Array_Contains` (`self.DetectedObjectSingles`) Object))
    (`KismetArrayLibrary.Array_Add` (`self.DetectedObjectSingles`) Object)))

(fn `RemoveDetectedObject`
  (params (Object :type "/Game/Blueprints/Components/TurretDetectableComponent Object Reference") (Turret :type "/Game/Blueprints/Turrets/BaseTurret Object Reference"))
  (locals (indexToRemove :type Integer))
  (for _index (range (`KismetArrayLibrary.Array_Length` (`self.AllDetectedObjects`)))
    (if (== (`|GetArrayItem` (`self.AllDetectedObjects`) _index) Object)
      (set `local.indexToRemove` _index)
      (break)))
  (`KismetArrayLibrary.Array_Remove` (`self.AllDetectedObjects`) (`local.indexToRemove`))
  (if (not (`KismetArrayLibrary.Array_Contains` (`self.AllDetectedObjects`) Object))
    (`KismetArrayLibrary.Array_RemoveItem` (`self.DetectedObjectSingles`) Object)
    (`/Game/Blueprints/GameMaster/GameMaster.OnAllTurretsLostObject` (`/Game/Blueprints/Libraries/CommonLibrary.GetGameMaster`) Object Turret)))

(fn `SetupEvents`
  (add `/Game/Blueprints/GameMaster/GameMaster.OnTurretDectectedObject` (`/Game/Blueprints/Libraries/CommonLibrary.GetGameMaster`) (`|CreateDelegate` :!event `OnObjectDetected`))
  (add `/Game/Blueprints/GameMaster/GameMaster.OnTurretLostObject` (`/Game/Blueprints/Libraries/CommonLibrary.GetGameMaster`) (`|CreateDelegate` :!event `OnObjectLost`))
  (add `/Game/Blueprints/GameMaster/GameMaster.OnAllTurretsLostObject` (`/Game/Blueprints/Libraries/CommonLibrary.GetGameMaster`) (`|CreateDelegate` :!event `OnAllTurretsLosrtObject`)))

(fn `UserConstructionScript`)