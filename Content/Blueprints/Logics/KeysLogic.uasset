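; KeysLogic tracks the Key actors in the level and signals when all of them have been picked up.
; On BeginPlay it binds to the GameMaster's key events and gathers every Key actor into an array.
; Each pickup removes that key from the array, and emptying it makes the GameMaster call its all-keys-picked-up event.
; Its own OnAllKeyPickedUp handler is empty.
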(event `self.ReceiveBeginPlay`
  (`self.SetupEvents`)
  (`self.RegisterKeys`))

(event `OnKeyPickedUp`
  (params (Key :type "/Game/Blueprints/Actors/Key Object Reference"))
  (if (`KismetArrayLibrary.Array_Contains` (`self.Keys`) Key)
    (`KismetArrayLibrary.Array_RemoveItem` (`self.Keys`) Key)
    (if (== (`KismetArrayLibrary.Array_Length` (`self.Keys`)) 0)
      (`/Game/Blueprints/GameMaster/GameMaster.OnAllKeysPickedUp` (`/Game/Blueprints/Libraries/CommonLibrary.GetGameMaster`)))))

(event `OnAllKeyPickedUp`)

(fn `RegisterKeys`
  (bind _outactors (`GameplayStatics.GetAllActorsOfClass` "/Game/Blueprints/Actors/Key.Key_C"))
  (set `self.Keys` _outactors))

(fn `SetupEvents`
  (add `/Game/Blueprints/GameMaster/GameMaster.OnKeyPickedUp` (`/Game/Blueprints/Libraries/CommonLibrary.GetGameMaster`) (`|CreateDelegate` :!event `OnKeyPickedUp`))
  (add `/Game/Blueprints/GameMaster/GameMaster.OnAllKeysPickedUp` (`/Game/Blueprints/Libraries/CommonLibrary.GetGameMaster`) (`|CreateDelegate` :!event `OnAllKeyPickedUp`)))

(fn `UserConstructionScript`)