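; PlayerRadarLogic drives the player's objective radar, showing a world-space pointer toward each enabled objective.
; It binds to GameMaster events to store the player camera and to spawn or destroy a PlayerRadarPointer per objective component, tracked as pointer-component pairs.
; Every tick, it places each pointer a fixed distance from the camera along the objective's direction, rotates it to face back, and updates its widget with the distance in meters.
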(event `self.ReceiveBeginPlay`
  (`self.SetupEvents`))

(event `self.ReceiveTick`
  (params (DeltaSeconds :type "Float (single-precision)"))
  (`self.ManagePointers`))

(event `OnPlayerCameraSetup`
  (params (Camera :type "SceneComponent Object Reference"))
  (set `self.PlayerCamera` Camera))

(event `OnObjectiveEnabled`
  (params (Actor :type "Actor Object Reference") (Component :type "/Game/Blueprints/Components/RadarComponent Object Reference"))
  (bind _returnvalue (`|SpawnActorFromClass` "/Game/Blueprints/Player/PlayerRadarPointer.PlayerRadarPointer_C" (`KismetMathLibrary.MakeTransform` (`self.K2_GetActorLocation` Actor)) "Undefined" "OverrideRootScale" null (`/Game/Blueprints/Components/RadarComponent.Name` Component) "/Game/Textures/Dot.Dot" null))
  (`KismetArrayLibrary.Array_Add` (`self.PointerComponentPairs`) (make `/Game/Blueprints/Player/PlayerRadarPointerComponentPair` _returnvalue Component)))

(event `OnObjectiveDisabled`
  (params (Actor :type "Actor Object Reference") (Component :type "/Game/Blueprints/Components/RadarComponent Object Reference"))
  (for (_array_element _array_index) (`self.PointerComponentPairs`)
    (if (== (`.Component_5_3004D08746B15D66F192EAA98136D326` (break `/Game/Blueprints/Player/PlayerRadarPointerComponentPair` _array_element)) Component)
      (`self.K2_DestroyActor` (break `/Game/Blueprints/Player/PlayerRadarPointerComponentPair` _array_element))
      (`KismetArrayLibrary.Array_Remove` (`self.PointerComponentPairs`) _array_index)
      (break))))

(fn `ManagePointers`
  (bind _returnvalue (`SceneComponent.K2_GetComponentLocation` (`self.PlayerCamera`)))
  (for _array_element (`self.PointerComponentPairs`)
    (bind _returnvalue_2 (`self.K2_GetActorLocation` (`ActorComponent.GetOwner` (`.Component_5_3004D08746B15D66F192EAA98136D326` (break `/Game/Blueprints/Player/PlayerRadarPointerComponentPair` _array_element)))))
    (`SceneComponent.K2_SetWorldLocationAndRotation` (`/Game/Blueprints/Player/PlayerRadarPointer.DefaultSceneRoot` (break `/Game/Blueprints/Player/PlayerRadarPointerComponentPair` _array_element)) (+ _returnvalue (* (`KismetMathLibrary.Normal` (- _returnvalue_2 _returnvalue)) (`self.DistanceFromCamera`))) (`KismetMathLibrary.FindLookAtRotation` _returnvalue_2 _returnvalue) false false)
    (`/Game/Blueprints/Widgets/DetectionWidget.SetDistance` (`/Game/Blueprints/Player/PlayerRadarPointer.RadarWidget` (break `/Game/Blueprints/Player/PlayerRadarPointerComponentPair` _array_element)) (`KismetStringLibrary.Conv_IntToString` (`KismetMathLibrary.FFloor` (* (`KismetMathLibrary.Vector_Distance` _returnvalue_2 _returnvalue) 0.01))))))

(fn `SetupEvents`
  (add `/Game/Blueprints/GameMaster/GameMaster.OnPlayerRadarObjEnabled` (`/Game/Blueprints/Libraries/CommonLibrary.GetGameMaster`) (`|CreateDelegate` :!event `OnObjectiveEnabled`))
  (add `/Game/Blueprints/GameMaster/GameMaster.OnPlayerRadarObjDisabled` (`/Game/Blueprints/Libraries/CommonLibrary.GetGameMaster`) (`|CreateDelegate` :!event `OnObjectiveDisabled`))
  (add `/Game/Blueprints/GameMaster/GameMaster.OnPlayerCameraSetup` (`/Game/Blueprints/Libraries/CommonLibrary.GetGameMaster`) (`|CreateDelegate` :!event `OnPlayerCameraSetup`)))

(fn `UserConstructionScript`)