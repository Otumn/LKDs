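; UIButtonsLogic is a logic Blueprint that turns UI button presses into game flow actions.
; On BeginPlay it binds to the Game Master's OnUIButtonPressed event.
; A switch on button type routes Main Menu, Replay and Next Level to the matching Game Master calls, while Quit exits the game directly.
; The Game Master acts as the event hub for both incoming presses and outgoing requests.
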(event `self.ReceiveBeginPlay`
  (`self.SetupEvents`))

(event `OnButtonPressed`
  (params (Type :type "/Game/Blueprints/UI/UIButtonType Enum" :default "NewEnumerator0"))
  (switch `/Game/Blueprints/UI/UIButtonType` Type
    (:`NewEnumerator1`
      (`/Game/Blueprints/GameMaster/GameMaster.OnGoToMainMenu` (`/Game/Blueprints/Libraries/CommonLibrary.GetGameMaster`)))
    (:`NewEnumerator2`
      (`KismetSystemLibrary.QuitGame` null "Quit"))
    (:`NewEnumerator3`
      (`/Game/Blueprints/GameMaster/GameMaster.OnReplayLevel` (`/Game/Blueprints/Libraries/CommonLibrary.GetGameMaster`)))
    (:`NewEnumerator4`
      (`/Game/Blueprints/GameMaster/GameMaster.OnGoToNextLevel` (`/Game/Blueprints/Libraries/CommonLibrary.GetGameMaster`)))))

(fn `SetupEvents`
  (add `/Game/Blueprints/GameMaster/GameMaster.OnUIButtonPressed` (`/Game/Blueprints/Libraries/CommonLibrary.GetGameMaster`) (`|CreateDelegate` :!event `OnButtonPressed`)))

(fn `UserConstructionScript`)