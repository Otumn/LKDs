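; Logic Blueprint that handles picking up, dropping and throwing throwable actors for pawns.
; It binds to the GameMaster's throwable interaction event on BeginPlay, releasing the pawn's held actor if present, otherwise snapping the grabbed one to the grab root with physics off.
; Each actor's ThrowableComponent drives the release: optional rotation reset, physics state and a launch impulse divided by mass, applied as a velocity change.
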(event `self.ReceiveBeginPlay`
  (`self.SetupEvents`))

(event `OnThrowableInteraction`
  (params (GrabbedActor :type "Actor Object Reference") (Pawn :type "/Game/Blueprints/Player/FirstPersonCharacter Object Reference") (GrabRoot :type "SceneComponent Object Reference") (LaunchParam :type "/Game/Blueprints/Throwable/LaunchParameters Structure"))
  (bind _heldthrowableactor (`/Game/Blueprints/Player/FirstPersonCharacter.HeldThrowableActor` Pawn))
  (`/Engine/EditorBlueprintResources/StandardMacros.IsValid` _heldthrowableactor
    (:`Is Valid`
      (`self.ReleaseThrowable` Pawn (`self.GetComponentByClass` _heldthrowableactor "/Game/Blueprints/Components/ThrowableComponent.ThrowableComponent_C") _heldthrowableactor LaunchParam))
    (:`Is Not Valid`
      (`/Engine/EditorBlueprintResources/StandardMacros.IsValid` GrabbedActor
        (:`Is Valid`
          (`self.SnapThrowable` Pawn (`self.GetComponentByClass` GrabbedActor "/Game/Blueprints/Components/ThrowableComponent.ThrowableComponent_C") GrabbedActor GrabRoot))))))

(event `SnapThrowable`
  (params (Pawn :type "/Game/Blueprints/Player/FirstPersonCharacter Object Reference") (Component :type "/Game/Blueprints/Components/ThrowableComponent Object Reference") (Actor :type "Actor Object Reference") (Root :type "SceneComponent Object Reference"))
  (bind _output_get (set `/Game/Blueprints/Player/FirstPersonCharacter.HeldThrowableActor` Actor Pawn))
  (`PrimitiveComponent.SetSimulatePhysics` (`/Game/Blueprints/Components/ThrowableComponent.PhysicsParent` Component) false)
  (`self.K2_AttachToComponent` _output_get Root "None" "SnapToTarget" "SnapToTarget" "KeepWorld" true)
  (`/Game/Blueprints/Components/ThrowableComponent.OnGrabbed` Component))

(event `ReleaseThrowable`
  (params (Pawn :type "/Game/Blueprints/Player/FirstPersonCharacter Object Reference") (Component :type "/Game/Blueprints/Components/ThrowableComponent Object Reference") (Actor :type "Actor Object Reference") (LaunchParam :type "/Game/Blueprints/Throwable/LaunchParameters Structure"))
  (bind (_force _direction) (break `/Game/Blueprints/Throwable/LaunchParameters` LaunchParam))
  (bind _physicsparent (`/Game/Blueprints/Components/ThrowableComponent.PhysicsParent` Component))
  (set `/Game/Blueprints/Player/FirstPersonCharacter.HeldThrowableActor` null Pawn)
  (`self.K2_DetachFromActor` Actor "KeepWorld" "KeepWorld" "KeepWorld")
  (`|ExecutionSequence`
    (:`then_0`
      (if (`/Game/Blueprints/Components/ThrowableComponent.ResetRotationOnDrop` Component)
        (`self.K2_SetActorRotation` :`self` Actor)))
    (:`then_1`
      (`PrimitiveComponent.SetSimulatePhysics` _physicsparent (`/Game/Blueprints/Components/ThrowableComponent.SimulatePhysicsOnDrop` Component)))
    (:`then_2`
      (if (`/Game/Blueprints/Components/ThrowableComponent.ThrowOnDrop` Component)
        (`PrimitiveComponent.AddImpulse` _physicsparent (/ (* _direction _force) (`/Game/Blueprints/Components/ThrowableComponent.Mass` Component)) "None" true)))))

(fn `SetupEvents`
  (add `/Game/Blueprints/GameMaster/GameMaster.OnThrowableInteraction` (`/Game/Blueprints/Libraries/CommonLibrary.GetGameMaster`) (`|CreateDelegate` :!event `OnThrowableInteraction`)))

(fn `UserConstructionScript`)