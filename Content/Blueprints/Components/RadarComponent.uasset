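; Actor component that registers its owner as an object on the player's radar.
; Display and Hide events forward an actor and component to the GameMaster, which raises its radar object enabled or disabled calls.
; On BeginPlay it waits briefly, then displays the owner automatically if DisplayOnBeginPlay is set.
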(event `self.ReceiveBeginPlay`
  (`KismetSystemLibrary.Delay` 0.2)
  (if (`self.DisplayOnBeginPlay`)
    (`self.Display` (`self.GetOwner`) self)))

(event `Display`
  (params (Actor :type "Actor Object Reference") (Component :type "/Game/Blueprints/Components/RadarComponent Object Reference"))
  (`/Game/Blueprints/GameMaster/GameMaster.OnPlayerRadarObjEnabled` (`/Game/Blueprints/Libraries/CommonLibrary.GetGameMaster`) Actor Component))

(event `Hide`
  (params (Actor :type "Actor Object Reference") (Component :type "/Game/Blueprints/Components/RadarComponent Object Reference"))
  (`/Game/Blueprints/GameMaster/GameMaster.OnPlayerRadarObjDisabled` (`/Game/Blueprints/Libraries/CommonLibrary.GetGameMaster`) Actor Component))