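; Key pickup actor that spins and bobs in place, then homes in on the player to be collected.
; Each tick it rotates, and a timeline drives the vertical bob until the detection sphere catches a FirstPersonCharacter.
; It then moves toward that character's capsule at a set speed.
; Overlapping the pickup sphere notifies the GameMaster, hides its radar component and destroys the actor.
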(event `self.ReceiveBeginPlay`
  (set `self.InitialLocation` (`SceneComponent.K2_GetComponentLocation` (`self.DefaultSceneRoot`))))

(event `self.ReceiveTick`
  (params (DeltaSeconds :type "Float (single-precision)"))
  (set `self.DeltaTime` DeltaSeconds)
  (`self.Animate`)
  (`self.MoveToPlayer`))

(event `MoveToPlayer`
  (if (`KismetSystemLibrary.IsValid` (`self.Player`))
    (`SceneComponent.K2_AddWorldOffset` (`self.DefaultSceneRoot`) (* (`KismetMathLibrary.Normal` (- (`SceneComponent.K2_GetComponentLocation` (`Character.CapsuleComponent` (`self.Player`))) (`SceneComponent.K2_GetComponentLocation` (`self.DefaultSceneRoot`)))) (* (`self.DeltaTime`) (`self.Speed`))) false false)))

(event `Animate`
  (bind (_initiallocation_x _initiallocation_y _initiallocation_z) (`KismetMathLibrary.BreakVector` (`self.InitialLocation`)))
  (`SceneComponent.K2_AddWorldRotation` (`self.DefaultSceneRoot`) (`KismetMathLibrary.MakeRotator` 0.0 0.0 (`self.DeltaRotation`)) false false)
  (if (not (`KismetSystemLibrary.IsValid` (`self.Player`)))
    (bind (_direction _z) (`Timeline|Timeline_0` :!label _label)
      (:`Update`
        (`SceneComponent.K2_SetWorldLocation` (`self.DefaultSceneRoot`) (`KismetMathLibrary.MakeVector` _initiallocation_x _initiallocation_y (+ _initiallocation_z (* _z (`self.DeltaZ`)))) false false)))))

(event `self.PlayerDetectionSphere.OnComponentBeginOverlap`
  (params (OverlappedComponent :type "PrimitiveComponent Object Reference") (OtherActor :type "Actor Object Reference") (OtherComp :type "PrimitiveComponent Object Reference") (OtherBodyIndex :type Integer) (bFromSweep :type Boolean) (SweepResult :type "HitResult Structure (by ref)"))
  (bind _asfirst_person_character (cast `/Game/Blueprints/Player/FirstPersonCharacter` OtherActor))
  (set `self.Player` _asfirst_person_character)
  (goto _label :!via `Stop`))

(event `self.PickupSphere.OnComponentBeginOverlap`
  (params (OverlappedComponent :type "PrimitiveComponent Object Reference") (OtherActor :type "Actor Object Reference") (OtherComp :type "PrimitiveComponent Object Reference") (OtherBodyIndex :type Integer) (bFromSweep :type Boolean) (SweepResult :type "HitResult Structure (by ref)"))
  (cast `/Game/Blueprints/Player/FirstPersonCharacter` OtherActor)
  (`/Game/Blueprints/GameMaster/GameMaster.OnKeyPickedUp` (`/Game/Blueprints/Libraries/CommonLibrary.GetGameMaster`) self)
  (`/Game/Blueprints/Components/RadarComponent.Hide` (`self.RadarComponent`) self (`self.RadarComponent`))
  (`self.K2_DestroyActor`))

(fn `SetSpheresRadiuses`
  (`SphereComponent.SetSphereRadius` (`self.PickupSphere`) (`self.PickupSphereRadius`) true)
  (`SphereComponent.SetSphereRadius` (`self.PlayerDetectionSphere`) (`self.DetectionSphereRadius`) true))

(fn `UserConstructionScript`)