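; Level exit door that stays shut until the game master reports that all keys are picked up.
; It binds to the game master's key events at BeginPlay and disables its end trigger; the single-key handler is empty.
; Opening slides both halves to their open root positions, turns their dots and light green, and enables the trigger.
; When the first-person character overlaps that trigger, it notifies the game master that the door is reached.
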(event `self.ReceiveBeginPlay`
  (`self.SetupEvents`)
  (`PrimitiveComponent.SetCollisionEnabled` (`self.LevelEndCollision`) "NoCollision"))

(event `OnKeyPickedUp`
  (params (Key :type "/Game/Blueprints/Actors/Key Object Reference")))

(event `OnAllKeysPickedUp`
  (`self.Open`))

(event `Open`
  (`PrimitiveComponent.SetCollisionEnabled` (`self.LevelEndCollision`) "QueryAndPhysics")
  (`self.MoveLeftSide`)
  (`self.MoveRightSide`)
  (`self.SetOpennedColors`))

(event `MoveLeftSide`
  (`KismetSystemLibrary.MoveComponentTo` (`self.LeftSide`) (`SceneComponent.RelativeLocation` (`self.LeftSideOpenedRoot`)) (struct) false true))

(event `MoveRightSide`
  (`KismetSystemLibrary.MoveComponentTo` (`self.RightSide`) (`SceneComponent.RelativeLocation` (`self.RightSideOpenedRoot`)) (struct) false true))

(event `self.LevelEndCollision.OnComponentBeginOverlap`
  (params (OverlappedComponent :type "PrimitiveComponent Object Reference") (OtherActor :type "Actor Object Reference") (OtherComp :type "PrimitiveComponent Object Reference") (OtherBodyIndex :type Integer) (bFromSweep :type Boolean) (SweepResult :type "HitResult Structure (by ref)"))
  (cast `/Game/Blueprints/Player/FirstPersonCharacter` OtherActor)
  (`/Game/Blueprints/GameMaster/GameMaster.OnLevelEndDoorReached` (`/Game/Blueprints/Libraries/CommonLibrary.GetGameMaster`)))

(fn `SetOpennedColors`
  (`MeshComponent.SetVectorParameterValueOnMaterials` (`self.RightSide`) "DotsColor" (0.0 1.0 0.0))
  (`MeshComponent.SetVectorParameterValueOnMaterials` (`self.LeftSide`) "DotsColor" (0.0 1.0 0.0))
  (`LightComponent.SetLightColor` (`self.PointLight`) (struct :`R` 0.019408 :`G` 1.0 :`A` 1.0) true))

(fn `SetupEvents`
  (add `/Game/Blueprints/GameMaster/GameMaster.OnKeyPickedUp` (`/Game/Blueprints/Libraries/CommonLibrary.GetGameMaster`) (`|CreateDelegate` :!event `OnKeyPickedUp`))
  (add `/Game/Blueprints/GameMaster/GameMaster.OnAllKeysPickedUp` (`/Game/Blueprints/Libraries/CommonLibrary.GetGameMaster`) (`|CreateDelegate` :!event `OnAllKeysPickedUp`)))

(fn `UserConstructionScript`)