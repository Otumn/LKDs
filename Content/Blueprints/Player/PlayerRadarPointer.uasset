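; Player radar pointer Blueprint that labels a radar detection marker with a name and icon.
; On BeginPlay it gets the DetectionWidget from its Widget component through a cast helper, then passes its Name and Image variables to that widget.
; It holds no tracking or update logic; the construction script is empty.
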(event `self.ReceiveBeginPlay`
  (bind _output_get (set `self.RadarWidget` (`self.GetWidget`)))
  (`/Game/Blueprints/Widgets/DetectionWidget.SetName` _output_get (`self.Name`))
  (`/Game/Blueprints/Widgets/DetectionWidget.SetIcon` _output_get (`self.Image`)))

(fn `GetWidget`
  (returns (Widget :type "/Game/Blueprints/Widgets/DetectionWidget Object Reference"))
  (bind _asdetection_widget (cast `/Game/Blueprints/Widgets/DetectionWidget` (`WidgetComponent.GetUserWidgetObject` (`self.Widget`))))
  (return _asdetection_widget))

(fn `UserConstructionScript`)